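; BP_PlatformRef is a sprite-based platformer character with a name label and a defeat sequence.
; BeginPlay passes the character's name to its W_NameCharcters widget.
; Defeat runs once, disabling capsule collision and the movement plane constraint, then launching the character up and sideways by configurable amounts.
; It also jumps the animation state machine to the defeated node, plays a death sound and raises the sprite's translucent sort priority to draw on top.
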(event `self.ReceiveBeginPlay`
  (bind _asw_name_charcters (cast `/Game/UI/W_NameCharcters` (`WidgetComponent.GetWidget` (`self.Name`))))
  (`/Game/UI/W_NameCharcters.UpdateNameCharacter` _asw_name_charcters (`self.Name Character`)))

(event `Defeat`
  (if (not (`self.isDefeated`))
    (set `self.isDefeated` true)
    (`PrimitiveComponent.SetCollisionEnabled` (`self.CapsuleComponent`) "NoCollision")
    (`MovementComponent.SetPlaneConstraintEnabled` (`self.CharacterMovement`) false)
    (`self.Launchondefead`)
    (`PaperZDAnimInstance.JumpToNode` (`self.GetAnimInstance`) "JumpDefeated" "None")
    ;[1 1 1] Звук смерти
    (`GameplayStatics.PlaySound2D` "/Game/Sounds/PlayerDefeated/S_PlayerDefeated_Cue.S_PlayerDefeated_Cue" 1.0 1.0 0.0 null null)
    (`PrimitiveComponent.SetTranslucentSortPriority` (`self.Sprite`) 100000)))

(fn `Launchondefead`
  (`self.LaunchCharacter` (+ (* (`KismetMathLibrary.Vector_Up`) (`self.DefeadUpLaunch`)) (* (`KismetMathLibrary.Vector_Right`) (`self.DefeadForwardLaunch`))) true true))

(fn `UserConstructionScript`)