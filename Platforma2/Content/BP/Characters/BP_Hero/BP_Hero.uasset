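; BP_Hero is the side-scrolling platformer player character, handling X-axis movement, jumping, weapon cycling, quest item pickup and death.
; Weapon and quest item state live in PC_Platform, which the hero updates on input.
; Tick turns the controller toward travel direction and, while airborne, traces below the feet to toggle one-way platform collision.
; Defeat removes input, detaches the camera and plays sound and shake; enemy stomp logic is disconnected.
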(event `self.ReceiveTick`
  (params (DeltaSeconds :type "Float (single-precision)"))
  (`parent.ReceiveTick` DeltaSeconds)
  (`self.UpdateControlRotation`)
  (`self.TraceForPlatforms`))

(event `self.ReceiveBeginPlay`
  (`parent.ReceiveBeginPlay`) ; Берет все функции из родителя
  ;[1 1 1] Подключаем управление для персонажа
  (bind _aspc_platform (cast `/Game/BP/PC_Platform` (`self.GetController`)))
  (bind _output_get (set `self.Ref PC Platform` _aspc_platform))
  (`EnhancedInputSubsystemInterface.AddMappingContext` (pcsubsystem `EnhancedInputLocalPlayerSubsystem` _output_get) "/Game/BP/Imputs/IMC_Platformer.IMC_Platformer" 0 (struct)))

(event `EnhancedInput|/Game/BP/Imputs/Actions/IA_Jump`
  (params (ActionValue :type Boolean) (ElapsedSeconds :type "Float (double-precision)") (TriggeredSeconds :type "Float (double-precision)") (InputAction :type "InputAction Object Reference" :default "/Game/BP/Imputs/Actions/IA_Jump.IA_Jump"))
  ;[1 1 1] Анимация Прыжка
  (:`Started`
    (`self.Jump`))
  (:`Completed`
    (`self.StopJumping`)))

(event `EnhancedInput|/Game/BP/Imputs/Actions/IA_Move`
  (params (ActionValue :type "Float (double-precision)") (ElapsedSeconds :type "Float (double-precision)") (TriggeredSeconds :type "Float (double-precision)") (InputAction :type "InputAction Object Reference" :default "/Game/BP/Imputs/Actions/IA_Move.IA_Move"))
  ;[1 1 1] Анимация бега
  (:`Triggered`
    (`self.AddMovementInput` (1.0 0.0 0.0) ActionValue)))

(event `EnhancedInput|/Game/BP/Imputs/Actions/IA_SwapWeapon`
  (params (ActionValue :type Boolean) (ElapsedSeconds :type "Float (double-precision)") (TriggeredSeconds :type "Float (double-precision)") (InputAction :type "InputAction Object Reference" :default "/Game/BP/Imputs/Actions/IA_SwapWeapon.IA_SwapWeapon"))
  (bind _ref_pc_platform (`self.Ref PC Platform`))
  (bind _equipweapons_indexweapon (break `/Game/BP/Weapon/S_WeaponHero` (`/Game/BP/PC_Platform.EquipWeapons` _ref_pc_platform)))
  (bind _equipweapons_indexweapon_2 (break `/Game/BP/Weapon/S_WeaponHero` (`/Game/BP/PC_Platform.EquipWeapons` _ref_pc_platform)))
  (bind _equipweapons_indexweapon_3 (break `/Game/BP/Weapon/S_WeaponHero` (`/Game/BP/PC_Platform.EquipWeapons` _ref_pc_platform)))
  (bind _equipweapons_indexweapon_4 (break `/Game/BP/Weapon/S_WeaponHero` (`/Game/BP/PC_Platform.EquipWeapons` _ref_pc_platform)))
  ;[1 1 1] Смена Оружия
  (:`Started`
    (if (>= (`KismetArrayLibrary.Array_Length` (`/Game/BP/PC_Platform.AllWeaponHero` (`self.Ref PC Platform`))) 2)
      (switch `int` _equipweapons_indexweapon_4
        (:`0`
          (`/Game/BP/PC_Platform.UpdateWeapon` _ref_pc_platform (+ _equipweapons_indexweapon 1) :!label _label))
        (:`1`
          (if (== (`KismetArrayLibrary.Array_Length` (`/Game/BP/PC_Platform.AllWeaponHero` (`self.Ref PC Platform`))) 2)
            (`/Game/BP/PC_Platform.UpdateWeapon` _ref_pc_platform (- _equipweapons_indexweapon_2 1))
            (else
              (goto _label))))
        (:`2`
          (`/Game/BP/PC_Platform.UpdateWeapon` _ref_pc_platform (- _equipweapons_indexweapon_3 2))))
      (else
        (`KismetSystemLibrary.PrintString` "Нет оружия")))))

(event `EnhancedInput|/Game/BP/Imputs/Actions/IA_Equip_Drop`
  (params (ActionValue :type Boolean) (ElapsedSeconds :type "Float (double-precision)") (TriggeredSeconds :type "Float (double-precision)") (InputAction :type "InputAction Object Reference" :default "/Game/BP/Imputs/Actions/IA_Equip_Drop.IA_Equip_Drop"))
  (bind _equipquestitem_indexitem (break `/Game/Quest_System/S_QuestItem` (`/Game/BP/PC_Platform.EquipQuestItem` (`self.Ref PC Platform`))))
  ;[1 1 1] Подбираем/ Выбрасываем Квестовые предметы
  (:`Started`
    (if (== _equipquestitem_indexitem 0)
      (if (> (`KismetArrayLibrary.Array_Length` (`PrimitiveComponent.GetOverlappingActors` (`self.BoxUse`) "/Game/Quest_System/BP_QuestItem.BP_QuestItem_C")) 0)
        (bind _returnvalue (`GameplayStatics.GetActorOfClass` "/Game/Quest_System/BP_QuestItem.BP_QuestItem_C"))
        (`/Game/BP/PC_Platform.UpdateQuestItem` (`self.Ref PC Platform`) (`/Game/Quest_System/BP_QuestItem.ItemInfo` _returnvalue))
        (`self.K2_DestroyActor` _returnvalue)
        (else
          (`KismetSystemLibrary.PrintString` "Нет квест предмета" true true (struct :`R` 1.0 :`G` 0.109751 :`B` 0.050025 :`A` 1.0)))))))

(event `self.CapsuleComponent.OnComponentBeginOverlap`
  (params (OverlappedComponent :type "PrimitiveComponent Object Reference") (OtherActor :type "Actor Object Reference") (OtherComp :type "PrimitiveComponent Object Reference") (OtherBodyIndex :type Integer) (bFromSweep :type Boolean) (SweepResult :type "HitResult Structure (by ref)"))
  ;[1 1 1] Убийство Врага или Врагом
)

(event `self.Defeat`
  ;[1 1 1] Смерть Персонажа
  (`parent.Defeat`)
  ;;[1 1 1] Забираем управление персонажем после смерти. через удаление контроллера
  (bind _asplayer_controller (cast `PlayerController` (`self.GetController`)))
  (`EnhancedInputSubsystemInterface.RemoveMappingContext` (pcsubsystem `EnhancedInputLocalPlayerSubsystem` _asplayer_controller) "/Game/BP/Imputs/IMC_Platformer.IMC_Platformer" (struct))
  ;;[1 1 1] Отсоеденяем камеру от персонажа
  (`SceneComponent.K2_DetachFromComponent` (`self.SpringArm`) "KeepWorld" "KeepRelative" "KeepRelative" true)
  ;;[1 1 1] Звук смерти
  (`GameplayStatics.PlaySound2D` "/Game/Sounds/PlayerDefeated/S_PlayerDefeated_Cue.S_PlayerDefeated_Cue" 1.0 1.0 0.0 null null)
  ;;[1 1 1] Тряска камеры
  (`GameplayStatics.PlayWorldCameraShake` "/Game/CameraShake/Camera_Shake_Defeated.Camera_Shake_Defeated_C" (`self.K2_GetActorLocation`) 0.0 10000.0))

(fn `TraceForPlatforms`
  (bind (_returnvalue_x _returnvalue_y _returnvalue_z) (`KismetMathLibrary.BreakVector` (`self.GetVelocity`)))
  (bind _returnvalue (`SceneComponent.K2_GetComponentLocation` (`self.footPosition`)))
  (if (`NavMovementComponent.IsFalling` (`self.CharacterMovement`))
    (bind (_outhit _returnvalue_2) (`KismetSystemLibrary.LineTraceSingleForObjects` _returnvalue (+ _returnvalue (* (`KismetMathLibrary.Vector_Down`) (`self.PlatformerCheckDistance`))) (`|MakeArray` "ObjectTypeQuery7" :!type "EObjectTypeQuery Enum")))
    (if (and _returnvalue_2 (< _returnvalue_z 0.0))
      (`PrimitiveComponent.SetCollisionResponseToChannel` (`self.CapsuleComponent`) "ECC_GameTraceChannel1" "ECR_Block")
      (else
        (`PrimitiveComponent.SetCollisionResponseToChannel` (`self.CapsuleComponent`) "ECC_GameTraceChannel1" "ECR_Overlap")))))

(fn `UpdateControlRotation`
  (bind _returnvalue (`self.GetController`))
  (bind _returnvalue_2 (`self.GetController`))
  (bind _velocity_x (`KismetMathLibrary.BreakVector` (`MovementComponent.Velocity` (`self.CharacterMovement`))))
  (`/Engine/EditorBlueprintResources/StandardMacros.CompareFloat` _velocity_x
    (:`>`
      (`/Engine/EditorBlueprintResources/StandardMacros.IsValid` _returnvalue_2
        (:`Is Valid`
          (`Controller.SetControlRotation` _returnvalue_2 (`KismetMathLibrary.MakeRotator` 0.0)))))
    (:`<`
      (`/Engine/EditorBlueprintResources/StandardMacros.IsValid` _returnvalue
        (:`Is Valid`
          (`Controller.SetControlRotation` _returnvalue (`KismetMathLibrary.MakeRotator` 0.0 0.0 180.0)))))))

(fn `UserConstructionScript`
  (`parent.UserConstructionScript`))