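; BP_NPC is a character Blueprint for an NPC that shows a WidgetPressF prompt when something enters its TargetQuest zone.
; The prompt starts hidden and appears on begin overlap only if the entering actor itself overlaps a BP_Hero, rather than being cast to one.
; Any end overlap hides it without a filter, and debug prints mark entry and exit.
; No F-key handling or quest logic is present.
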(event `self.ReceiveBeginPlay`
  (`parent.ReceiveBeginPlay`)
  (`SceneComponent.SetVisibility` (`self.Widget_PressF`) false false))

(event `self.TargetQuest.OnComponentBeginOverlap`
  (params (OverlappedComponent :type "PrimitiveComponent Object Reference") (OtherActor :type "Actor Object Reference") (OtherComp :type "PrimitiveComponent Object Reference") (OtherBodyIndex :type Integer) (bFromSweep :type Boolean) (SweepResult :type "HitResult Structure (by ref)"))
  (if (> (`KismetArrayLibrary.Array_Length` (`self.GetOverlappingActors` OtherActor "/Game/BP/Characters/BP_Hero/BP_Hero.BP_Hero_C")) 0)
    (`SceneComponent.SetVisibility` (`self.Widget_PressF`) true false)
    (`KismetSystemLibrary.PrintString` "Вошли в зону Ф")))

(event `self.TargetQuest.OnComponentEndOverlap`
  (params (OverlappedComponent :type "PrimitiveComponent Object Reference") (OtherActor :type "Actor Object Reference") (OtherComp :type "PrimitiveComponent Object Reference") (OtherBodyIndex :type Integer))
  (`SceneComponent.SetVisibility` (`self.Widget_PressF`) false false)
  (`KismetSystemLibrary.PrintString` "Вышли из зоны Ф"))

(fn `UserConstructionScript`
  (`parent.UserConstructionScript`))