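; PC_Platform, likely a player controller, holds the hero's weapons, quest item, HP and stamina and shows them on the HUD.
; On BeginPlay it creates the W_HUD widget, then pushes weapon, health and stamina to its panels.
; Update events set weapon and quest icons, hiding the quest icon for index 0, and choose a slower stamina regen rate in combat.
; Adding a new weapon also equips it by its index.
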(event `self.ReceiveBeginPlay`
  (`self.StartGame`))

(event `StartGame`
  (`self.Visibility HUD`)
  (`self.UpdateWeapon` (`.IndexWeapon_20_97954F8D452EAA3DCB96D19A2961B681` (break `/Game/BP/Weapon/S_WeaponHero` (`self.EquipWeapons`))))
  (`self.UpdateHP`)
  (`self.UpdateStamina`))

(event `Visibility HUD`
  (bind _returnvalue (`|CreateWidget` "/Game/UI/Panel/W_HUD.W_HUD_C"))
  (bind _output_get (set `self.Ref W HUD` _returnvalue))
  (`UserWidget.AddToViewport` _output_get 0))

(event `UpdateWeapon`
  (params (IndexWeapon :type Integer :default 1))
  ;[1 1 1] ОРУЖИЕ
  (bind _output_get (set `self.EquipWeapons` (`|GetArrayItem` (`self.AllWeaponHero`) IndexWeapon)))
  (set `Image.Brush` (make `SlateBrush` "Image" "NoTile" "NoMirror" (struct :`X` 32.0 :`Y` 32.0) (struct) (struct :`SpecifiedColor` (struct :`R` 1.0 :`G` 1.0 :`B` 1.0 :`A` 1.0) :`ColorUseRule` "UseColor_Specified") (struct :`CornerRadii` (struct :`W` 1.0) :`Color` (struct :`SpecifiedColor` (struct) :`ColorUseRule` "UseColor_Specified") :`RoundingType` "HalfHeightRadius") (`.Icon_15_CC70C22B4207978868D812A792C26CD6` (break `/Game/BP/Weapon/S_WeaponHero` _output_get))) (`/Game/UI/Panel/W_Panel_Weapons.Image_Weapon` (`/Game/UI/Panel/W_HUD.W_Panel_Weapons` (`self.Ref W HUD`)))))

(event `UpdateQuestItem`
  (params (EquipQuestItem :type "/Game/Quest_System/S_QuestItem Structure"))
  (bind _image_quest_item (`/Game/UI/Quests/W_Panel_ItemQuest.Image_Quest_Item` (`/Game/UI/Panel/W_HUD.W_Panel_Quest` (`self.Ref W HUD`))))
  (bind _image_quest_item_2 (`/Game/UI/Quests/W_Panel_ItemQuest.Image_Quest_Item` (`/Game/UI/Panel/W_HUD.W_Panel_Quest` (`self.Ref W HUD`))))
  ;[1 1 1] Проверяем и обновляем информацию о квестовых предметах
  (if (== (`.IndexItem_7_8F774775465B17FD1076C7A09DEBD15C` (break `/Game/Quest_System/S_QuestItem` EquipQuestItem)) 0)
    (bind _output_get (set `self.EquipQuestItem` EquipQuestItem))
    (set `Image.Brush` (make `SlateBrush` "Image" "NoTile" "NoMirror" (struct :`X` 32.0 :`Y` 32.0) (struct) (struct :`SpecifiedColor` (struct :`R` 1.0 :`G` 1.0 :`B` 1.0 :`A` 1.0) :`ColorUseRule` "UseColor_Specified") (struct :`CornerRadii` (struct :`W` 1.0) :`Color` (struct :`SpecifiedColor` (struct) :`ColorUseRule` "UseColor_Specified") :`RoundingType` "HalfHeightRadius") (`.Icon_10_95C6D8ED48756900493ACD9955748CE8` (break `/Game/Quest_System/S_QuestItem` _output_get))) _image_quest_item)
    (set `Image.ColorAndOpacity` (make `LinearColor` 0.0) _image_quest_item)
    (else
      (bind _output_get_2 (set `self.EquipQuestItem` EquipQuestItem))
      (set `Image.Brush` (make `SlateBrush` "Image" "NoTile" "NoMirror" (struct :`X` 32.0 :`Y` 32.0) (struct) (struct :`SpecifiedColor` (struct :`R` 1.0 :`G` 1.0 :`B` 1.0 :`A` 1.0) :`ColorUseRule` "UseColor_Specified") (struct :`CornerRadii` (struct :`W` 1.0) :`Color` (struct :`SpecifiedColor` (struct) :`ColorUseRule` "UseColor_Specified") :`RoundingType` "HalfHeightRadius") (`.Icon_10_95C6D8ED48756900493ACD9955748CE8` (break `/Game/Quest_System/S_QuestItem` _output_get_2))) _image_quest_item_2)
      (set `Image.ColorAndOpacity` (make `LinearColor` 1.0 1.0 1.0 1.0) _image_quest_item_2))))

(event `ADDWeaponHero`
  (params (NewWeapon :type "/Game/BP/Weapon/S_WeaponHero Structure (by ref)"))
  ;[1 1 1] ОРУЖИЕ
  (if (not (`KismetArrayLibrary.Array_Contains` (`self.AllWeaponHero`) NewWeapon))
    (`KismetArrayLibrary.Array_Add` (`self.AllWeaponHero`) NewWeapon)
    (`self.UpdateWeapon` (`.IndexWeapon_20_97954F8D452EAA3DCB96D19A2961B681` (break `/Game/BP/Weapon/S_WeaponHero` NewWeapon)))))

(event `UpdateHP`
  ;[1 1 1] Здоровье Персонажа
  (`/Game/UI/Panel/W_Panel_HP.UpdateHPBar` (`/Game/UI/Panel/W_HUD.W_Panel_HP` (`self.Ref W HUD`)) (`self.HP`)))

(event `UpdateStamina`
  (bind _w_panel_stamina (`/Game/UI/Panel/W_HUD.W_Panel_Stamina` (`self.Ref W HUD`)))
  ;[1 1 1] Обновляем Выносливость персонажа в бою и вне боя
  (if (`self.HeroFight`)
    (bind _output_get (set `self.PowerRegen` 0.01)) ; Скорость регенерации в бою
    (`/Game/UI/Panel/W_Panel_Stamina.UpdateStaminaBar` _w_panel_stamina (`self.Stamina`) _output_get)
    (else
      (bind _output_get_2 (set `self.PowerRegen` 0.2)) ; Скорость регенерации вне боя
      (`/Game/UI/Panel/W_Panel_Stamina.UpdateStaminaBar` _w_panel_stamina (`self.Stamina`) _output_get_2))))

(fn `UserConstructionScript`)